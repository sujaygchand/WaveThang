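; Spawn manager that populates the level with AI pirate and navy ships on BeginPlay.
; ShipSpawner loops over an index range, spawning the given pawn class with the pirate ship behavior tree, which both factions share.
; Helper functions supply random placement within bounds set by marker actors, with random yaw and height taken from the X-max marker.
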(event EventActorBeginOverlap
  (params (OtherActor :type Actor%20Object%20Reference)))

(event EventTick
  (params (DeltaSeconds :type Float%20%28single-precision%29)))

(event EventBeginPlay
  (Variables|Default|SetNewActorTransform (Utilities|SetNewRandomTransformation))
  (CallFunction|ShipSpawner 0 4 "/Game/AI/Pawns/AIPirateShip.AIPirateShip_C")
  (CallFunction|ShipSpawner 0 7 "/Game/AI/Pawns/AINavyShip.AINavyShip_C"))

(fn ConstructionScript)

(fn ShipSpawner
  (params (First%20Index :type Integer) (Last%20Index :type Integer) (ShipType1 :type Pawn%20Class%20Reference))
  (bind _returnvalue (Utilities|SetNewRandomTransformation))
  ;[1 1 1] Spawns SHips and creates array with new location
  (for _index (range First%20Index Last%20Index)
    (bind _output_get (LocalVariables|SetShipType ShipType1))
    (AI|SpawnAIFromClass _output_get "/Game/AI/BT_PirateShip.BT_PirateShip" (.location _returnvalue) (.rotation _returnvalue) false))
  (return))