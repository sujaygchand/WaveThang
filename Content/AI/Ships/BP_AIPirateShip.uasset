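; AI pirate ship Blueprint that picks a random island point at BeginPlay as its travel target.
; The RandomiseTarget macro gathers all BP_IslandPoints actors and returns one at a random index.
; Tick calls GoToIsland every frame, which stores the target's location and calls MoveComponentTo; the trailing five-second Delay gates nothing.
; The target is never re-rolled, and a look-at rotation node is left unused.
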(event `self.ReceiveBeginPlay`
  ;[1 1 1] Initial random Choice
  (bind _target_island (`self.RandomiseTarget`)
    (:`true`
      (set `self.TargetIsland` _target_island))))

(event `self.ReceiveTick`
  (params (DeltaSeconds :type "Float (single-precision)"))
  (`self.GoToIsland`)
  (`KismetSystemLibrary.Delay` 5.0))

(event `GoToIsland`
  (set `self.IslandLocation` (`self.K2_GetActorLocation` (`self.TargetIsland`)))
  (`KismetSystemLibrary.MoveComponentTo` null))

(fn `UserConstructionScript`
  (`parent.UserConstructionScript`))